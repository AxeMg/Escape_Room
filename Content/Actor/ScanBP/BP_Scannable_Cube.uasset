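; Scannable cube actor that highlights when scanned and can then be interacted with for a limited time.
; Activate turns on custom depth with a stencil value, presumably for a post-process outline, and marks the cube clickable until a delay clears both.
; Interact, while clickable, plays a timeline that pitches the cube mesh through a quarter turn.
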(event `Activate`
  (bind _cube (`self.Cube`))
  (`PrimitiveComponent.SetRenderCustomDepth` _cube true)
  (`PrimitiveComponent.SetCustomDepthStencilValue` _cube (`self.StencilValue`))
  (set `self.IsClickable` true)
  (`KismetSystemLibrary.Delay` 10.0)
  (`PrimitiveComponent.SetRenderCustomDepth` _cube false)
  (set `self.IsClickable` false))

(event `/Game/ThirdPerson/BPI_Interact.Interact`
  (if (`self.IsClickable`)
    (bind (_direction _newtrack_0) (`Timeline|Rotation`)
      (:`Update`
        (`SceneComponent.K2_SetRelativeRotation` (`self.Cube`) (`KismetMathLibrary.MakeRotator` 0.0 (`KismetMathLibrary.Lerp` 0.0 90.0 _newtrack_0)) false false)))))

(fn `UserConstructionScript`)