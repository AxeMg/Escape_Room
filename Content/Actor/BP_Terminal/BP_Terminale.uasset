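; BP_Terminale is an interactable terminal actor that opens the WB_Symbole widget when the player is inside its Box trigger.
; Box overlaps set a detection flag that gates Interact, which toggles on the player character's IsInteractive state.
; Entering shows the cursor, blocks movement, creates the widget and switches the view target to CameraRef.
; Exiting removes the widget and restores movement, cursor and player view.
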(event `/Game/ThirdPerson/BPI_Interact.Interact`
  (params (Player :type "/Game/ThirdPerson/Blueprints/BP_ThirdPersonCharacter Object Reference"))
  (bind _playerref (`self.PlayerRef`))
  (bind _playerref_2 (`self.PlayerRef`))
  (if (`self.IsDetect`)
    (`KismetSystemLibrary.PrintString` "Hello")
    (set `PlayerController.bShowMouseCursor` true (`GameplayStatics.GetPlayerController` 0))
    (set `/Game/ThirdPerson/Blueprints/BP_ThirdPersonCharacter.CanMoove` false _playerref)
    (if (and (`self.IsDetect`) (not (`/Game/ThirdPerson/Blueprints/BP_ThirdPersonCharacter.IsInteractive` _playerref)))
      (bind _returnvalue (`|CreateWidget` "/Game/Actor/BP_Terminal/LumièreEnigme/WB_Symbole.WB_Symbole_C"))
      (bind _output_get (set `self.WidgetRef` _returnvalue))
      (`UserWidget.AddToViewport` _output_get 0)
      (set `/Game/ThirdPerson/Blueprints/BP_ThirdPersonCharacter.IsInteractive` true (`self.PlayerRef`))
      (`PlayerController.SetViewTargetWithBlend` (`GameplayStatics.GetPlayerController` 0) (`self.CameraRef`) 0.0 "VTBlend_Linear" 0.0 false)
      (else
        (`Widget.RemoveFromParent` (`self.WidgetRef`))
        (set `self.IsDetect` true)
        (set `/Game/ThirdPerson/Blueprints/BP_ThirdPersonCharacter.IsInteractive` false _playerref_2)
        (set `/Game/ThirdPerson/Blueprints/BP_ThirdPersonCharacter.CanMoove` true _playerref_2)
        (set `PlayerController.bShowMouseCursor` false (`GameplayStatics.GetPlayerController` 0))
        (`PlayerController.SetViewTargetWithBlend` (`GameplayStatics.GetPlayerController` 0) (`GameplayStatics.GetPlayerCharacter` 0) 0.0 "VTBlend_Linear" 0.0 false)))))

(event `self.Box.OnComponentBeginOverlap`
  (params (OverlappedComponent :type "PrimitiveComponent Object Reference") (OtherActor :type "Actor Object Reference") (OtherComp :type "PrimitiveComponent Object Reference") (OtherBodyIndex :type Integer) (bFromSweep :type Boolean) (SweepResult :type "HitResult Structure (by ref)"))
  (set `self.IsDetect` true))

(event `self.Box.OnComponentEndOverlap`
  (params (OverlappedComponent :type "PrimitiveComponent Object Reference") (OtherActor :type "Actor Object Reference") (OtherComp :type "PrimitiveComponent Object Reference") (OtherBodyIndex :type Integer))
  (set `self.IsDetect` false))

(event `self.ReceiveBeginPlay`
  (bind _asbp_third_person_character (cast `/Game/ThirdPerson/Blueprints/BP_ThirdPersonCharacter` (`GameplayStatics.GetPlayerCharacter` 0)))
  (set `self.PlayerRef` _asbp_third_person_character))

(fn `UserConstructionScript`)