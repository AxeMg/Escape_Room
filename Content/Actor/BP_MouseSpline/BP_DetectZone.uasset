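; BP_DetectZone is a three-zone detector that shows whether BP_MouseSpline actors occupy each of its slider trigger components.
; All zones start red and unlit; an overlap turns the matching cube green, lights its spot and point lights and plays a sound.
; Leaving a zone reverts its cube and lights.
; Each entry sets a flag and runs a shared check, which currently only prints a debug string when all three are occupied.
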(event `self.ReceiveBeginPlay`
  (`PrimitiveComponent.SetMaterial` (`self.Cube_01`) 1 "/Game/Materials/Lights/MI_Light_Red.MI_Light_Red")
  (`PrimitiveComponent.SetMaterial` (`self.Cube_02`) 1 "/Game/Materials/Lights/MI_Light_Red.MI_Light_Red")
  (`PrimitiveComponent.SetMaterial` (`self.Cube_03`) 1 "/Game/Materials/Lights/MI_Light_Red.MI_Light_Red")
  (`LightComponent.SetIntensity` (`self.PointLight2`) 0.0)
  (`LightComponent.SetIntensity` (`self.PointLight1`) 0.0)
  (`LightComponent.SetIntensity` (`self.PointLight`) 0.0)
  (`LightComponent.SetIntensity` (`self.SpotLight_02`) 0.0)
  (`LightComponent.SetIntensity` (`self.SpotLight_01`) 0.0)
  (`LightComponent.SetIntensity` (`self.SpotLight_03`) 0.0))

(event `self.Slider_01.OnComponentBeginOverlap`
  (params (OverlappedComponent :type "PrimitiveComponent Object Reference") (OtherActor :type "Actor Object Reference") (OtherComp :type "PrimitiveComponent Object Reference") (OtherBodyIndex :type Integer) (bFromSweep :type Boolean) (SweepResult :type "HitResult Structure (by ref)"))
  (cast `/Game/Actor/BP_MouseSpline/BP_MouseSpline` OtherActor)
  (set `self.Cube_01_In` true)
  (`PrimitiveComponent.SetMaterial` (`self.Cube_01`) 1 "/Game/Materials/Lights/MI_Light_Green.MI_Light_Green")
  (`LightComponent.SetIntensity` (`self.SpotLight_01`) 250.0)
  (`LightComponent.SetIntensity` (`self.PointLight`) 400.0)
  (`GameplayStatics.PlaySoundAtLocation` "/Game/SFX/AmbiantEffect/the-sound-of-a-spotlight-in-a-room-with-an-echo_Cue.the-sound-of-a-spotlight-in-a-room-with-an-echo_Cue" (`self.K2_GetActorLocation`) (struct) 1.0 1.0 0.0 null null null null)
  (`self.3 cube In` :!label _label))

(event `self.Slider_02.OnComponentBeginOverlap`
  (params (OverlappedComponent :type "PrimitiveComponent Object Reference") (OtherActor :type "Actor Object Reference") (OtherComp :type "PrimitiveComponent Object Reference") (OtherBodyIndex :type Integer) (bFromSweep :type Boolean) (SweepResult :type "HitResult Structure (by ref)"))
  (cast `/Game/Actor/BP_MouseSpline/BP_MouseSpline` OtherActor)
  (set `self.Cube_02_In` true)
  (`PrimitiveComponent.SetMaterial` (`self.Cube_02`) 1 "/Game/Materials/Lights/MI_Light_Green.MI_Light_Green")
  (`LightComponent.SetIntensity` (`self.SpotLight_02`) 250.0)
  (`LightComponent.SetIntensity` (`self.PointLight1`) 400.0)
  (`GameplayStatics.PlaySoundAtLocation` "/Game/SFX/AmbiantEffect/the-sound-of-a-spotlight-in-a-room-with-an-echo_Cue.the-sound-of-a-spotlight-in-a-room-with-an-echo_Cue" (`self.K2_GetActorLocation`) (struct) 1.0 1.0 0.0 null null null null)
  (goto _label))

(event `self.Slider_03.OnComponentBeginOverlap`
  (params (OverlappedComponent :type "PrimitiveComponent Object Reference") (OtherActor :type "Actor Object Reference") (OtherComp :type "PrimitiveComponent Object Reference") (OtherBodyIndex :type Integer) (bFromSweep :type Boolean) (SweepResult :type "HitResult Structure (by ref)"))
  (cast `/Game/Actor/BP_MouseSpline/BP_MouseSpline` OtherActor)
  (set `self.Cube_03_In` true)
  (`PrimitiveComponent.SetMaterial` (`self.Cube_03`) 1 "/Game/Materials/Lights/MI_Light_Green.MI_Light_Green")
  (`LightComponent.SetIntensity` (`self.SpotLight_03`) 250.0)
  (`LightComponent.SetIntensity` (`self.PointLight2`) 400.0)
  (`GameplayStatics.PlaySoundAtLocation` "/Game/SFX/AmbiantEffect/the-sound-of-a-spotlight-in-a-room-with-an-echo_Cue.the-sound-of-a-spotlight-in-a-room-with-an-echo_Cue" (`self.K2_GetActorLocation`) (struct) 1.0 1.0 0.0 null null null null)
  (goto _label))

(event `self.Slider_01.OnComponentEndOverlap`
  (params (OverlappedComponent :type "PrimitiveComponent Object Reference") (OtherActor :type "Actor Object Reference") (OtherComp :type "PrimitiveComponent Object Reference") (OtherBodyIndex :type Integer))
  (cast `/Game/Actor/BP_MouseSpline/BP_MouseSpline` OtherActor)
  (set `self.Cube_01_In` false)
  (`PrimitiveComponent.SetMaterial` (`self.Cube_01`) 1 "/Game/Materials/Lights/MI_Light_Red.MI_Light_Red")
  (`LightComponent.SetIntensity` (`self.SpotLight_01`) 0.0)
  (`LightComponent.SetIntensity` (`self.PointLight`) 0.0))

(event `self.Slider_02.OnComponentEndOverlap`
  (params (OverlappedComponent :type "PrimitiveComponent Object Reference") (OtherActor :type "Actor Object Reference") (OtherComp :type "PrimitiveComponent Object Reference") (OtherBodyIndex :type Integer))
  (cast `/Game/Actor/BP_MouseSpline/BP_MouseSpline` OtherActor)
  (set `self.Cube_02_In` false)
  (`PrimitiveComponent.SetMaterial` (`self.Cube_02`) 1 "/Game/Materials/Lights/MI_Light_Red.MI_Light_Red")
  (`LightComponent.SetIntensity` (`self.SpotLight_02`) 0.0)
  (`LightComponent.SetIntensity` (`self.PointLight1`) 0.0))

(event `self.Slider_03.OnComponentEndOverlap`
  (params (OverlappedComponent :type "PrimitiveComponent Object Reference") (OtherActor :type "Actor Object Reference") (OtherComp :type "PrimitiveComponent Object Reference") (OtherBodyIndex :type Integer))
  (cast `/Game/Actor/BP_MouseSpline/BP_MouseSpline` OtherActor)
  (set `self.Cube_03_In` false)
  (`PrimitiveComponent.SetMaterial` (`self.Cube_03`) 1 "/Game/Materials/Lights/MI_Light_Red.MI_Light_Red")
  (`LightComponent.SetIntensity` (`self.SpotLight_03`) 0.0)
  (`LightComponent.SetIntensity` (`self.PointLight2`) 0.0))

(event `3 cube In`
  (if (and (and (`self.Cube_01_In`) (`self.Cube_02_In`)) (`self.Cube_03_In`))
    (`KismetSystemLibrary.PrintString` "WAZAAAAAAAAAAAAA")))

(fn `UserConstructionScript`)