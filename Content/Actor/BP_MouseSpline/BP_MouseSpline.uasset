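; Puzzle-style interactable whose cube the player click-drags along a spline, with optional hidden start and spotlight.
; While held, Tick projects mouse velocity through camera axes onto the spline direction, using the stronger of forward or up mapping, to advance distance.
; The character's click-release event ends dragging, and an overlay outlines the hovered or held cube in InteractMode.
; Activate highlights it temporarily via custom-depth stencil; the spline-mesh construction code is disconnected.
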(event `Activate`
  (bind _cubemesh (`self.CubeMesh`))
  (`PrimitiveComponent.SetRenderCustomDepth` _cubemesh true)
  (`PrimitiveComponent.SetCustomDepthStencilValue` _cubemesh (`self.StencilValue`))
  (`KismetSystemLibrary.Delay` 10.0)
  (`PrimitiveComponent.SetRenderCustomDepth` _cubemesh false))

(event `self.ReceiveBeginPlay`
  (bind _asbp_third_person_character (cast `/Game/ThirdPerson/Blueprints/BP_ThirdPersonCharacter` (`GameplayStatics.GetPlayerCharacter` 0)))
  (set `self.PlayerRef` _asbp_third_person_character)
  (add `/Game/ThirdPerson/Blueprints/BP_ThirdPersonCharacter.ClickRelease` _asbp_third_person_character (delegate `CustomEvent`))
  (if (`self.IsHiden`)
    (`self.SetActorHiddenInGame` true)))

(event `CustomEvent`
  (set `self.Clicked` false))

(event `/Game/CelyanTest/BPI_TestBPI.ToggleVisibilty`
  (`KismetSystemLibrary.PrintString` "Hello")
  (`self.SetActorHiddenInGame` false))

(event `self.ReceiveTick`
  (params (DeltaSeconds :type "Float (single-precision)"))
  (bind _playerref (`self.PlayerRef`))
  (bind _returnvalue (`SplineComponent.GetDirectionAtDistanceAlongSpline` (`self.Spline`) (`self.CurrentDist`) "World"))
  (bind _followcamera (`/Game/ThirdPerson/Blueprints/BP_ThirdPersonCharacter.FollowCamera` _playerref))
  (bind (_returnvalue_x _returnvalue_y) (`KismetMathLibrary.BreakVector2D` (`KismetMathLibrary.Normal2D` (`/Game/ThirdPerson/Blueprints/BP_ThirdPersonCharacter.MouseVelocity` _playerref))))
  (bind _returnvalue_2 (* (`SceneComponent.GetRightVector` _followcamera) _returnvalue_x))
  (bind _returnvalue_3 (`KismetMathLibrary.Dot_VectorVector` (`KismetMathLibrary.Normal` (+ (* (`SceneComponent.GetUpVector` _followcamera) _returnvalue_y -1.0) _returnvalue_2)) _returnvalue))
  (bind _returnvalue_4 (`KismetMathLibrary.Dot_VectorVector` (`KismetMathLibrary.Normal` (+ (* (`SceneComponent.GetForwardVector` _followcamera) _returnvalue_y -1.0) _returnvalue_2)) _returnvalue))
  (`self.Outline`)
  (if (and (`self.Clicked`) (`GameplayStatics.BreakHitResult` (`PlayerController.GetHitResultUnderCursorForObjects` (`GameplayStatics.GetPlayerController` 0) (`|MakeArray` "ObjectTypeQuery1" :!type "EObjectTypeQuery Enum") true)))
    (`SceneComponent.K2_SetWorldLocation` (`self.CubeMesh`) (`SplineComponent.GetLocationAtDistanceAlongSpline` (`self.Spline`) (`self.CurrentDist`) "World") false false)
    (set `self.CurrentDist` (+ (`self.CurrentDist`) (* (select `bool` (>= (`KismetMathLibrary.Abs` _returnvalue_4) (`KismetMathLibrary.Abs` _returnvalue_3)) :`false` _returnvalue_3 :`true` _returnvalue_4) (`self.Speed`))))))

(event `self.CubeMesh.OnClicked`
  (params (TouchedComponent :type "PrimitiveComponent Object Reference") (ButtonPressed :type "Key Structure"))
  (set `self.Clicked` true))

(event `Outline`
  ;[1 1 1] Outline
  (if (and (or (`self.Clicked`) (== (`self.CubeMesh`) (`.HitComponent` (`GameplayStatics.BreakHitResult` (`PlayerController.GetHitResultUnderCursorForObjects` (`GameplayStatics.GetPlayerController` 0) (`|MakeArray` "ObjectTypeQuery1" :!type "EObjectTypeQuery Enum") true))))) (`/Game/ThirdPerson/Blueprints/BP_ThirdPersonCharacter.InteractMode` (cast `/Game/ThirdPerson/Blueprints/BP_ThirdPersonCharacter` (`GameplayStatics.GetPlayerPawn` 0) :!pure true)))
    (`MeshComponent.SetOverlayMaterial` (`self.CubeMesh`) "/Game/Materials/Trash/MI_OutlineObject.MI_OutlineObject")
    (else
      (`MeshComponent.SetOverlayMaterial` (`self.CubeMesh`) null))))

(fn `UserConstructionScript`
  (if (`self.IsLightOn`)
    (`SceneComponent.SetVisibility` (`self.SpotLight`) true false)
    (else
      (`SceneComponent.SetVisibility` (`self.SpotLight`) false false))))