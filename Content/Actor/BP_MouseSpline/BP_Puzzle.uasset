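; Puzzle actor that is solved when BP_MouseSpline actors overlap all seven of its trigger boxes at once.
; Each box's begin and end overlap sets or clears its own flag, then re-runs PathCheck.
; When every flag is set, it lights the point light, marks IsValid and briefly blends the view to CameraValid before returning to the player character.
; Otherwise, it switches the light off; IsValid is never cleared here.
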(event `self.Box.OnComponentBeginOverlap`
  (params (OverlappedComponent :type "PrimitiveComponent Object Reference") (OtherActor :type "Actor Object Reference") (OtherComp :type "PrimitiveComponent Object Reference") (OtherBodyIndex :type Integer) (bFromSweep :type Boolean) (SweepResult :type "HitResult Structure (by ref)"))
  (cast `/Game/Actor/BP_MouseSpline/BP_MouseSpline` OtherActor)
  (set `self.IsBoxIn_01` true)
  (`self.PathCheck` :!label _label)
  (`KismetSystemLibrary.PrintString` "In"))

(event `self.Box1.OnComponentBeginOverlap`
  (params (OverlappedComponent :type "PrimitiveComponent Object Reference") (OtherActor :type "Actor Object Reference") (OtherComp :type "PrimitiveComponent Object Reference") (OtherBodyIndex :type Integer) (bFromSweep :type Boolean) (SweepResult :type "HitResult Structure (by ref)"))
  (cast `/Game/Actor/BP_MouseSpline/BP_MouseSpline` OtherActor)
  (set `self.IsBoxIn_02` true)
  (goto _label))

(event `self.Box2.OnComponentBeginOverlap`
  (params (OverlappedComponent :type "PrimitiveComponent Object Reference") (OtherActor :type "Actor Object Reference") (OtherComp :type "PrimitiveComponent Object Reference") (OtherBodyIndex :type Integer) (bFromSweep :type Boolean) (SweepResult :type "HitResult Structure (by ref)"))
  (cast `/Game/Actor/BP_MouseSpline/BP_MouseSpline` OtherActor)
  (set `self.IsBoxIn_03` true)
  (goto _label))

(event `self.Box3.OnComponentBeginOverlap`
  (params (OverlappedComponent :type "PrimitiveComponent Object Reference") (OtherActor :type "Actor Object Reference") (OtherComp :type "PrimitiveComponent Object Reference") (OtherBodyIndex :type Integer) (bFromSweep :type Boolean) (SweepResult :type "HitResult Structure (by ref)"))
  (cast `/Game/Actor/BP_MouseSpline/BP_MouseSpline` OtherActor)
  (set `self.IsBoxIn_04` true)
  (goto _label))

(event `self.Box4.OnComponentBeginOverlap`
  (params (OverlappedComponent :type "PrimitiveComponent Object Reference") (OtherActor :type "Actor Object Reference") (OtherComp :type "PrimitiveComponent Object Reference") (OtherBodyIndex :type Integer) (bFromSweep :type Boolean) (SweepResult :type "HitResult Structure (by ref)"))
  (cast `/Game/Actor/BP_MouseSpline/BP_MouseSpline` OtherActor)
  (set `self.IsBoxIn_05` true)
  (goto _label))

(event `self.Box5.OnComponentBeginOverlap`
  (params (OverlappedComponent :type "PrimitiveComponent Object Reference") (OtherActor :type "Actor Object Reference") (OtherComp :type "PrimitiveComponent Object Reference") (OtherBodyIndex :type Integer) (bFromSweep :type Boolean) (SweepResult :type "HitResult Structure (by ref)"))
  (cast `/Game/Actor/BP_MouseSpline/BP_MouseSpline` OtherActor)
  (set `self.IsBoxIn_06` true)
  (goto _label))

(event `PathCheck`
  (if (and (`self.IsBoxIn_01`) (`self.IsBoxIn_02`) (`self.IsBoxIn_03`) (`self.IsBoxIn_04`) (`self.IsBoxIn_05`) (`self.IsBoxIn_06`) (`self.IsBoxIn_07`))
    (`KismetSystemLibrary.PrintString` "HeOIUIOOIllo")
    (`LightComponent.SetIntensity` (`self.PointLight`) 5000.0)
    (set `self.IsValid` true)
    (`PlayerController.SetViewTargetWithBlend` (`GameplayStatics.GetPlayerController` 0) (`self.CameraValid`) 0.5 "VTBlend_EaseIn" 0.0 false)
    (`KismetSystemLibrary.Delay` 3.0)
    (`PlayerController.SetViewTargetWithBlend` (`GameplayStatics.GetPlayerController` 0) (`GameplayStatics.GetPlayerCharacter` 0) 0.3 "VTBlend_EaseOut" 0.0 false)
    (else
      (`LightComponent.SetIntensity` (`self.PointLight`) 0.0))))

(event `self.Box6.OnComponentBeginOverlap`
  (params (OverlappedComponent :type "PrimitiveComponent Object Reference") (OtherActor :type "Actor Object Reference") (OtherComp :type "PrimitiveComponent Object Reference") (OtherBodyIndex :type Integer) (bFromSweep :type Boolean) (SweepResult :type "HitResult Structure (by ref)"))
  (cast `/Game/Actor/BP_MouseSpline/BP_MouseSpline` OtherActor)
  (set `self.IsBoxIn_07` true)
  (goto _label))

(event `self.Box.OnComponentEndOverlap`
  (params (OverlappedComponent :type "PrimitiveComponent Object Reference") (OtherActor :type "Actor Object Reference") (OtherComp :type "PrimitiveComponent Object Reference") (OtherBodyIndex :type Integer))
  (cast `/Game/Actor/BP_MouseSpline/BP_MouseSpline` OtherActor)
  (set `self.IsBoxIn_01` false)
  (`self.PathCheck` :!label _label_2)
  (`KismetSystemLibrary.PrintString` "Out"))

(event `self.Box1.OnComponentEndOverlap`
  (params (OverlappedComponent :type "PrimitiveComponent Object Reference") (OtherActor :type "Actor Object Reference") (OtherComp :type "PrimitiveComponent Object Reference") (OtherBodyIndex :type Integer))
  (cast `/Game/Actor/BP_MouseSpline/BP_MouseSpline` OtherActor)
  (set `self.IsBoxIn_02` false)
  (goto _label_2))

(event `self.Box2.OnComponentEndOverlap`
  (params (OverlappedComponent :type "PrimitiveComponent Object Reference") (OtherActor :type "Actor Object Reference") (OtherComp :type "PrimitiveComponent Object Reference") (OtherBodyIndex :type Integer))
  (cast `/Game/Actor/BP_MouseSpline/BP_MouseSpline` OtherActor)
  (set `self.IsBoxIn_03` false)
  (goto _label_2))

(event `self.Box3.OnComponentEndOverlap`
  (params (OverlappedComponent :type "PrimitiveComponent Object Reference") (OtherActor :type "Actor Object Reference") (OtherComp :type "PrimitiveComponent Object Reference") (OtherBodyIndex :type Integer))
  (cast `/Game/Actor/BP_MouseSpline/BP_MouseSpline` OtherActor)
  (set `self.IsBoxIn_04` false)
  (goto _label_2))

(event `self.Box4.OnComponentEndOverlap`
  (params (OverlappedComponent :type "PrimitiveComponent Object Reference") (OtherActor :type "Actor Object Reference") (OtherComp :type "PrimitiveComponent Object Reference") (OtherBodyIndex :type Integer))
  (cast `/Game/Actor/BP_MouseSpline/BP_MouseSpline` OtherActor)
  (set `self.IsBoxIn_05` false)
  (goto _label_2))

(event `self.Box5.OnComponentEndOverlap`
  (params (OverlappedComponent :type "PrimitiveComponent Object Reference") (OtherActor :type "Actor Object Reference") (OtherComp :type "PrimitiveComponent Object Reference") (OtherBodyIndex :type Integer))
  (cast `/Game/Actor/BP_MouseSpline/BP_MouseSpline` OtherActor)
  (set `self.IsBoxIn_06` false)
  (goto _label_2))

(event `self.Box6.OnComponentEndOverlap`
  (params (OverlappedComponent :type "PrimitiveComponent Object Reference") (OtherActor :type "Actor Object Reference") (OtherComp :type "PrimitiveComponent Object Reference") (OtherBodyIndex :type Integer))
  (cast `/Game/Actor/BP_MouseSpline/BP_MouseSpline` OtherActor)
  (set `self.IsBoxIn_07` false)
  (goto _label_2))

(fn `UserConstructionScript`)