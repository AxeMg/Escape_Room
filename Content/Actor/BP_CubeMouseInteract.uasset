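; BP_CubeMouseInteract is a cube actor that the player pushes around with mouse movement.
; Each Tick calls SetActorTransform, then, if the third-person character's CanTakeTheCube is true and CanCameraMove is false, applies mouse delta as a velocity-change impulse.
; Inverted mouse X drives world X and mouse Y drives Z, while Interact runs the same check.
; BeginPlay caches a BP_Spline reference that the graph never reads.
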(event `self.ReceiveTick`
  (params (DeltaSeconds :type "Float (single-precision)"))
  (bind _staticmeshcomponent0 (`self.StaticMeshComponent0`))
  (bind (_deltax _deltay) (`PlayerController.GetInputMouseDelta` (`GameplayStatics.GetPlayerController` 0)))
  (bind _asbp_third_person_character (cast `/Game/ThirdPerson/Blueprints/BP_ThirdPersonCharacter` (`GameplayStatics.GetPlayerCharacter` 0) :!pure true))
  (bind (_relativelocation_x _relativelocation_y _relativelocation_z) (`KismetMathLibrary.BreakVector` (`SceneComponent.RelativeLocation` _staticmeshcomponent0)))
  (`self.K2_SetActorTransform` (`KismetMathLibrary.MakeTransform` (0.0 0.0 0.0)))
  (if (and (`/Game/ThirdPerson/Blueprints/BP_ThirdPersonCharacter.CanTakeTheCube` _asbp_third_person_character) (not (`/Game/ThirdPerson/Blueprints/BP_ThirdPersonCharacter.CanCameraMove` _asbp_third_person_character))) :!label _label
    (`PrimitiveComponent.AddVelocityChangeImpulseAtLocation` _staticmeshcomponent0 (`KismetMathLibrary.MakeVector` (* (* _deltax 100.0) -1.0) 0.0 (* _deltay 100.0)) (`KismetMathLibrary.MakeVector` _relativelocation_x _relativelocation_y _relativelocation_z) "None")))

(event `self.ReceiveBeginPlay`
  (bind _returnvalue (`GameplayStatics.GetActorOfClass` "/Game/Actor/BP_Spline.BP_Spline_C"))
  (set `self.Spline REF` _returnvalue))

(event `/Game/ThirdPerson/BPI_Interact.Interact`
  (goto _label))

(fn `UserConstructionScript`)