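; BP_Doure is an automatic double sliding door that opens while something overlaps its Box trigger.
; Begin overlap plays the Ouverture timeline and end overlap reverses it, with no filter on the overlapping actor.
; The timeline's Speed track drives Lerps that slide the left and right panels apart in opposite directions along relative X.
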(event `self.Box.OnComponentBeginOverlap`
  (params (OverlappedComponent :type "PrimitiveComponent Object Reference") (OtherActor :type "Actor Object Reference") (OtherComp :type "PrimitiveComponent Object Reference") (OtherBodyIndex :type Integer) (bFromSweep :type Boolean) (SweepResult :type "HitResult Structure (by ref)"))
  (bind (_direction _speed) (`Timeline|Ouverture` :!label _label)
    (:`Update`
      (`SceneComponent.K2_SetRelativeLocation` (`self.SM_Porte_PorteGauche2_StaticMeshComponent0`) (`KismetMathLibrary.MakeVector` (`KismetMathLibrary.Lerp` 0.0 -65.0 _speed)) false false)
      (`SceneComponent.K2_SetRelativeLocation` (`self.SM_Porte_PorteDroite2_StaticMeshComponent0`) (`KismetMathLibrary.MakeVector` (`KismetMathLibrary.Lerp` 0.0 65.0 _speed)) false false))))

(event `self.Box.OnComponentEndOverlap`
  (params (OverlappedComponent :type "PrimitiveComponent Object Reference") (OtherActor :type "Actor Object Reference") (OtherComp :type "PrimitiveComponent Object Reference") (OtherBodyIndex :type Integer))
  (goto _label :!via `Reverse`))

(fn `UserConstructionScript`)